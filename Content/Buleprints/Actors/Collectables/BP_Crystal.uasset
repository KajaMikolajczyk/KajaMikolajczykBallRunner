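; BP_Crystal is a collectable crystal that flies into the player and vanishes when the player pawn overlaps its SphereTrigger.
; On overlap it caches its location and PointLight intensity, then plays the CrystalMovement timeline.
; The timeline's curves lerp it toward the pawn's current position, fade the light and drive the disappearing scale, then the actor destroys itself.
; No score or inventory update happens here, and the collision-disabling branch is unconnected.
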(event `self.ReceiveActorBeginOverlap`
  (params (OtherActor :type "Actor Object Reference")))

(event `self.SphereTrigger.OnComponentBeginOverlap`
  (params (OverlappedComponent :type "PrimitiveComponent Object Reference") (OtherActor :type "Actor Object Reference") (OtherComp :type "PrimitiveComponent Object Reference") (OtherBodyIndex :type Integer) (bFromSweep :type Boolean) (SweepResult :type "HitResult Structure (by ref)"))
  (`/Game/Buleprints/Libraries/ML_Actors.IsPlayer` OtherActor
    (:`IsPlayer`
      (`self.Location`)
      (`self.LerpBasicIntensity`)
      (bind (_direction _smoothlerpalpha _light_intensity _scale) (`Timeline|CrystalMovement`)
        (:`Update`
          (`self.Light` _light_intensity)
          (`self.DisappearingCrystalScale` _scale)
          (`self.CrystalMovementTorwardsPlayer` _smoothlerpalpha (`GameplayStatics.GetPlayerPawn` 0)))
        (:`Finished`
          (`self.K2_DestroyActor`))))))

(fn `CrystalMovementTorwardsPlayer`
  (params (Alpha :type "Float (double-precision)") (self2 :type "Actor Object Reference"))
  (`self.K2_SetActorLocation` (`KismetMathLibrary.VLerp` (`self.LerpStartLocation`) (`self.K2_GetActorLocation` self2) Alpha)))

(fn `DisappearingCrystalScale`
  (params (Alpha :type "Float (double-precision)"))
  (`self.SetActorScale3D` (`KismetMathLibrary.VLerp` (0.0 0.0 0.0) (1.0 1.0 1.0) Alpha)))

(fn `LerpBasicIntensity`
  (set `self.LerpStartIntensity` (`LightComponentBase.Intensity` (`self.PointLight`))))

(fn `Light`
  (params (NewIntensity :type "Float (double-precision)"))
  (`LightComponent.SetIntensity` (`self.PointLight`) (`KismetMathLibrary.Lerp` (`self.LerpStartIntensity`) 0.0 NewIntensity)))

(fn `Location`
  (set `self.LerpStartLocation` (`self.K2_GetActorLocation`)))

(fn `UserConstructionScript`)