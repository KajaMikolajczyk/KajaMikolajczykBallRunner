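; BP_BackToStart is a trigger actor that sends the player back to a start location while crystals remain in the level.
; On overlap, an IsPlayer check filters the actor, then CheckAnyCrystals counts all BP_Crystal actors.
; CheckAnyCrystals returns true when none are left, despite its name; otherwise player pawn 0 is moved to PlayerStart without sweep.
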(event `self.ReceiveActorBeginOverlap`
  (params (OtherActor :type "Actor Object Reference"))
  (`/Game/Buleprints/Libraries/ML_Actors.IsPlayer` OtherActor
    (:`IsPlayer`
      (if (not (`self.CheckAnyCrystals`))
        (`self.K2_SetActorLocation` (`GameplayStatics.GetPlayerPawn` 0) (`self.PlayerStart`) false false)))))

(fn `CheckAnyCrystals`
  (returns (ReturnValue :type Boolean))
  (bind _outactors (`GameplayStatics.GetAllActorsOfClass` "/Game/Buleprints/Actors/Collectables/BP_Crystal.BP_Crystal_C"))
  (return (== (`KismetArrayLibrary.Array_Length` _outactors) 0)))

(fn `UserConstructionScript`)