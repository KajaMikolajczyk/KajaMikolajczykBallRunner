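; BP_WinVolume is a volume that completes the level when the player overlaps it and no BP_Crystal actors remain in the world.
; On completion it finds the current level's name in the LevelsNames array to get its index.
; It then opens the next entry by name, or quits the game if the current level is the last one in the array.
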(event `self.ReceiveActorBeginOverlap`
  (params (OtherActor :type "Actor Object Reference"))
  (`/Game/Buleprints/Libraries/ML_Actors.IsPlayer` OtherActor
    (:`IsPlayer`
      (if (`self.CheckAnyCrystals`)
        (`self.CompleteLevel`)))))

(fn `CheckAnyCrystals`
  (returns (ReturnValue :type Boolean))
  (bind _outactors (`GameplayStatics.GetAllActorsOfClass` "/Game/Buleprints/Actors/Collectables/BP_Crystal.BP_Crystal_C"))
  (return (== (`KismetArrayLibrary.Array_Length` _outactors) 0)))

(fn `CompleteLevel`
  (bind _returnvalue (`self.GetCurrentLevelIndex`))
  (if (== (`self.IsFinalLvl`) _returnvalue)
    (`KismetSystemLibrary.QuitGame` null "Quit")
    (else
      (`self.LoadNextLevel` _returnvalue))))

(fn `GetCurrentLevelIndex`
  (returns (ReturnValue :type Integer))
  (bind _returnvalue (`GameplayStatics.GetCurrentLevelName` true))
  (return (`KismetArrayLibrary.Array_Find` (`self.LevelsNames`) (`KismetStringLibrary.Conv_StringToName` _returnvalue))))

(fn `GetNextLevelName`
  (params (CurrentLevelName :type Integer))
  (returns (Output :type "Name (by ref)"))
  (return (`|GetArrayItem` (`self.LevelsNames`) (+ CurrentLevelName 1))))

(fn `IsFinalLvl`
  (returns (ReturnValue :type Integer))
  (return (`KismetArrayLibrary.Array_LastIndex` (`self.LevelsNames`))))

(fn `LoadNextLevel`
  (params (A :type Integer))
  (`GameplayStatics.OpenLevel` (`self.GetNextLevelName` A)))

(fn `UserConstructionScript`)