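; BP_Player2 is a player pawn that rolls a sphere with physics torque and restarts the level when it takes damage.
; Both movement axes trigger one shared mass-independent torque node, which applies the same scaled axis value to X and Y.
; Any damage, regardless of amount, runs YouAreDead, which starts a camera fade, waits briefly, then reopens the current level by name.
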(event `InputAxis|Move Forward_Backwards`
  (params (AxisValue :type "Float (single-precision)"))
  (`PrimitiveComponent.AddTorqueInRadians` (`self.Sphere`) (`KismetMathLibrary.MakeVector` (* (stale `InputAxis|Move Left_Right` AxisValue) (`self.Torque Strenght`)) (* AxisValue (`self.Torque Strenght`))) "None" true :!label _label))

(event `InputAxis|Move Left_Right`
  (params (AxisValue :type "Float (single-precision)"))
  (goto _label))

(event `self.ReceiveAnyDamage`
  (params (Damage :type "Float (single-precision)") (DamageType :type "DamageType Object Reference") (InstigatedBy :type "Controller Object Reference") (DamageCauser :type "Actor Object Reference"))
  (`self.YouAreDead!`))

(fn `UserConstructionScript`)